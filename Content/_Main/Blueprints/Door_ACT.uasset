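; Door actor that swings open when its trigger box is overlapped, provided the player character's CanEnter flag is set.
; The DoorUpDown_ANIM timeline scales the Rotation variable to drive the Cube's relative yaw, and reverses when the overlap ends.
; Otherwise it prints a message telling the player to collect all the coins.
; The gate reads player 0's character rather than checking which actor overlapped.
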(event OnComponentBeginOverlap(Box)
  (params (OverlappedComponent :type Primitive%20Component%20Object%20Reference) (OtherActor :type Actor%20Object%20Reference) (OtherComp :type Primitive%20Component%20Object%20Reference) (OtherBodyIndex :type Integer) (bFromSweep :type Boolean) (SweepResult :type Hit%20Result%20Structure%20%28by%20ref%29))
  (bind _asthird_person_character (Utilities|Casting|CastToThirdPersonCharacter (Game|GetPlayerCharacter 0)))
  (if (Variables|/Game/ThirdPersonBP/Blueprints/ThirdPersonCharacter.ThirdPersonCharacter_C|GetCanEnter _asthird_person_character)
    (Development|PrintString "Door Opened!" true true "(R=0.278894,G=0.000000,B=1.000000,A=1.000000)" 5.0)
    (bind _up (Timeline|DoorUpDown_ANIM Play)
      (:Update
        (Transformation|SetRelativeRotation (Variables|Default|GetCube) (Math|Rotator|MakeRotator 0.0 0.0 (* _up (Variables|Default|GetRotation))) false false)))
    (else
      (Development|PrintString "Collect all the Coins!" true true "(R=0.278894,G=0.000000,B=1.000000,A=1.000000)" 5.0))))

(event OnComponentEndOverlap(Box)
  (params (OverlappedComponent :type Primitive%20Component%20Object%20Reference) (OtherActor :type Actor%20Object%20Reference) (OtherComp :type Primitive%20Component%20Object%20Reference) (OtherBodyIndex :type Integer))
  (bind _up (Timeline|DoorUpDown_ANIM Reverse)
    (:Update
      (Transformation|SetRelativeRotation (Variables|Default|GetCube) (Math|Rotator|MakeRotator 0.0 0.0 (* _up (Variables|Default|GetRotation))) false false))))

(fn ConstructionScript)