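; BP_Button is a proximity button that sends FloatingIsland to a fixed location.
; Overlapping its Box sets CanClick on both the button and the player's BP_SteveCharacter, and ending the overlap clears it.
; Tick polls the character's Pressed flag, without checking the button's own CanClick, then runs a timed MoveComponentTo on FloatingIsland followed by DestroyActor on the button.
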(event OnComponentBeginOverlap(Box)
  (params (OverlappedComponent :type Primitive%20Component%20Object%20Reference) (OtherActor :type Actor%20Object%20Reference) (OtherComp :type Primitive%20Component%20Object%20Reference) (OtherBodyIndex :type Integer) (bFromSweep :type Boolean) (SweepResult :type Hit%20Result%20Structure%20%28by%20ref%29))
  (Variables|Default|SetcanClick true)
  (bind _asbp_steve_character (Utilities|Casting|CastToBP_SteveCharacter (Game|GetPlayerCharacter 0)))
  (Variables|/Game/_Main/Blueprints/Character/BP_SteveCharacter.BP_SteveCharacter_C|SetcanClick _asbp_steve_character true))

(event OnComponentEndOverlap(Box)
  (params (OverlappedComponent :type Primitive%20Component%20Object%20Reference) (OtherActor :type Actor%20Object%20Reference) (OtherComp :type Primitive%20Component%20Object%20Reference) (OtherBodyIndex :type Integer))
  (Variables|Default|SetcanClick false)
  (bind _asbp_steve_character (Utilities|Casting|CastToBP_SteveCharacter (Game|GetPlayerCharacter 0)))
  (Variables|/Game/_Main/Blueprints/Character/BP_SteveCharacter.BP_SteveCharacter_C|SetcanClick _asbp_steve_character false))

(event EventTick
  (params (DeltaSeconds :type Float%20%28single-precision%29))
  (bind _asbp_steve_character (Utilities|Casting|CastToBP_SteveCharacter (Game|GetPlayerCharacter 0)))
  (if (Variables|/Game/_Main/Blueprints/Character/BP_SteveCharacter.BP_SteveCharacter_C|GetPressed _asbp_steve_character)
    (Components|MoveComponentTo (Variables|Default|GetFloatingIsland) "29900.000000,-8.000000,52.000000" "0, 0,0.000000" false false 1e+01 false)
    (Actor|DestroyActor)))

(fn ConstructionScript)